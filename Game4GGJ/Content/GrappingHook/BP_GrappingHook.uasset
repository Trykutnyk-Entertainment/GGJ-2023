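; BP_GrappingHook is a grappling hook actor that shows a cable and pulls the main character toward the hooked point.
; doHook spawns an anchor sphere at the grab point, attached to the hit actor or, in the component variant, a Moving_Platform's Cube, and attaches the cable end to it.
; HookTick adds force toward the sphere, blended with left/right input for steering, or stops the hook when the sphere is invalid.
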(event Custom|doHook
  (params (GrabPoint :type Vector) (HitPoint :type Vector) (HitActor :type Actor%20Object%20Reference))
  (Audio|SpawnSound2D "/Game/GrappingHook/sounds/HOOK_PICKUP.HOOK_PICKUP" 1.0 1.0 0.0 0)
  (Rendering|SetVisibility (Variables|Default|GetCable) true false)
  (bind _returnvalue (Game|SpawnActorfromClass "/Game/GrappingHook/someSphere.someSphere_C" (Transformation|GetActorTransform) "Undefined" 0 0))
  (bind _output_get (Variables|Default|Setsphere _returnvalue))
  (Transformation|SetActorLocationAndRotation _output_get GrabPoint (Math|Rotator|MakeRotfromX HitPoint))
  (Transformation|AttachActorToActor (Variables|Default|Getsphere) HitActor "None" "KeepWorld" "KeepWorld" "KeepWorld" true)
  (Class|CableComponent|SetAttachEndto (Variables|Default|GetCable) (Variables|Default|Getsphere) (Variables|Default|GetComponent%20Property) (Variables|Default|GetCenter)))

(event Custom|stopHook
  (bind _sphere (Variables|Default|Getsphere))
  (Rendering|SetVisibility (Variables|Default|GetCable) false false)
  (Utilities|IsValid _sphere
    (:Is%20Valid
      (Actor|DestroyActor _sphere))))

(event Custom|HookTick
  (params (End%20Location :type Vector) (Character :type BP%20Main%20Character%20Object%20Reference))
  (bind _sphere (Variables|Default|Getsphere))
  (bind _output_get (Variables|Default|SetCharacter Character))
  (Utilities|IsValid _sphere
    (:Is%20Valid
      (bind _asbp_main_character (Utilities|Casting|CastToBP_MainCharacter _output_get))
      (Physics|AddForce (Variables|/Script/Engine.Character|GetCharacterMovement _asbp_main_character) (* (Math|Vector|Normalize (+ (Math|Vector|GetUnitDirection(Vector) (Transformation|GetActorLocation (Variables|Default|GetCharacter)) (Transformation|GetWorldLocation (Variables|/Script/Engine.Actor|GetRootComponent _sphere))) (* (* (Transformation|GetActorRightVector (Variables|Default|GetCharacter)) (Input|AxisValues|GetMoveLeft/Right)) 0.7))) 3.5e+05)))
    (:Is%20Not%20Valid
      (CallFunction|StopHook)
      (Variables|/Game/FirstPerson/Blueprints/BP_MainCharacter.BP_MainCharacter_C|SetisGrapping (Variables|Default|GetCharacter) false))))

(event Custom|doHook%28component%29
  (params (Grab%20Point :type Vector) (HitPoint :type Vector) (HitActor :type Actor%20Object%20Reference))
  (Rendering|SetVisibility (Variables|Default|GetCable) true false)
  (bind _returnvalue (Game|SpawnActorfromClass "/Game/GrappingHook/someSphere.someSphere_C" (Transformation|GetActorTransform) "Undefined" 0 0))
  (bind _asmoving_platform (Utilities|Casting|CastToMoving_Platform HitActor))
  (bind _output_get (Variables|Default|Setsphere _returnvalue))
  (Transformation|SetActorLocationAndRotation _output_get Grab%20Point (Math|Rotator|MakeRotfromX HitPoint))
  (Transformation|AttachComponentToComponent (Variables|Default|Getsphere) (Variables|/Game/LevelPrototyping/Meshes/Moving_Platform.Moving_Platform_C|GetCube _asmoving_platform) "None" "KeepWorld" "KeepWorld" "KeepWorld" true)
  (Class|CableComponent|SetAttachEndto (Variables|Default|GetCable) (Variables|Default|Getsphere) (Variables|Default|GetComponent%20Property) (Variables|Default|GetCenter)))

(fn ConstructionScript)