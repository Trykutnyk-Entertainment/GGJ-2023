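; GI_Discord is a game instance that integrates Discord Rich Presence into the game.
; Init creates and initializes a DiscordRpc object with the application ID, and Shutdown clears the presence.
; Rich Presence writes State and Details into the presence struct and pushes the update, with RichPresence as a wrapper.
; ChangeState updates the presence and caches the state, while SetDetailsLevel only caches the details text.
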(event EventInit
  (bind _returnvalue (Game|ConstructObjectfromClass "/Script/DiscordRpc.DiscordRpc"))
  (bind _output_get (Variables|Default|SetDiscordRPC _returnvalue))
  (Class|DiscordRpc|Initialize _output_get (Variables|Default|GetApplication%20Id) false))

(event EventShutdown
  (Class|DiscordRpc|ClearPresence (Variables|Default|GetDiscordRPC)))

(event EventSetDetailsLevel
  (params (Details :type String))
  (Variables|Default|SetDetails%20NOW Details))

(fn RichPresence
  (params (State :type String) (Details :type String))
  (bind _discordrpc (Variables|Default|GetDiscordRPC))
  (bind _structout (Utilities|Struct|SetmembersinDiscordRichPresence (Variables|/Script/DiscordRpc.DiscordRpc|GetRichPresence (Variables|Default|GetDiscordRPC)) State Details))
  (Variables|/Script/DiscordRpc.DiscordRpc|SetRichPresence _discordrpc _structout)
  (Class|DiscordRpc|UpdatePresence _discordrpc)
  (return true))

(fn ChangeState
  (params (State :type String) (Details :type String))
  (Discord|RichPresence State Details)
  (Variables|Default|SetState%20NOW State)
  (return false))

(fn RichPresence
  (params (State :type String) (Details :type String))
  (bind _returnvalue (Discord|RichPresence State Details))
  (return _returnvalue))