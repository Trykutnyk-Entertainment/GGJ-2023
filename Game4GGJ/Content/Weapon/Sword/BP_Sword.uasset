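; BP_Sword is a melee weapon that damages AI enemies and destroys homing carrot projectiles.
; Start and stop events toggle the sword's collision, with the start event storing the wielding player.
; Each overlapped actor is hit only once per activation via a TargetHit list cleared on stop.
; Hitting an AI_MAIN enemy applies fixed damage and grants the main character ammo.
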(event OnComponentBeginOverlap(swordCollision)
  (params (OverlappedComponent :type Primitive%20Component%20Object%20Reference) (OtherActor :type Actor%20Object%20Reference) (OtherComp :type Primitive%20Component%20Object%20Reference) (OtherBodyIndex :type Integer) (bFromSweep :type Boolean) (SweepResult :type Hit%20Result%20Structure%20%28by%20ref%29))
  (bind _targethit (Variables|Default|GetTargetHit))
  (bind _returnvalue (Utilities|Array|ContainsItem _targethit OtherActor))
  (bind _output_get (Variables|Default|SetHittedActor (Utilities|GetClass OtherActor)))
  (if (Utilities|ClassIsChildOf _output_get "/Game/ptaxalv/AI_MAIN.AI_MAIN_C")
    (if (not _returnvalue)
      (Utilities|Array|Add _targethit OtherActor)
      (Game|Damage|ApplyDamage OtherActor 2.0 0 0)
      (bind _asbp_main_character (Utilities|Casting|CastToBP_MainCharacter (Variables|Default|GetPlayer)))
      (Default|AddAmmo _asbp_main_character))
    (elif (Utilities|ClassIsChildOf _output_get "/Game/ptaxalv/GlowMat/HomingCarrot.HomingCarrot_C")
      (if (not _returnvalue)
        (Utilities|Array|Add _targethit OtherActor)
        (Utilities|IsValid OtherActor
          (:Is%20Valid
            (Actor|DestroyActor OtherActor)))))))

(event Custom|startOverlap
  (params (Player :type Actor%20Object%20Reference))
  (Variables|Default|SetPlayer Player)
  (Collision|SetCollisionProfileName (Variables|Default|GetswordCollision) "OverlapAll" true :!class /Script/Engine.PrimitiveComponent))

(event Custom|stopOverlap
  (Collision|SetCollisionEnabled (Variables|Default|GetswordCollision) "NoCollision")
  (Utilities|Array|Clear (Variables|Default|GetTargetHit)))

(fn ConstructionScript)